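; Player-controlled helicopter pawn that flies, looks around with the mouse and fires bullets.
; On possession it adds the player input mapping context, feeding movement actions into FloatingPawnMovement along world X/Y and mouse input into controller yaw and pitch.
; Two RotatingMovement components, bound at BeginPlay, spin RotorBase and Sphere4.
; Primary fire spawns BP_Bullet at the Projectile1 transform after a short delay.
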(event Custom|SetRotatingParts
  (Components|Movement|SetUpdatedComponent (Variables|Default|GetRotatingMovement) (Variables|Default|GetRotorBase))
  (Components|Movement|SetUpdatedComponent (Variables|Default|GetRotatingMovement1) (Variables|Default|GetSphere4)))

(event Custom|RotatePlayerPawnYAW)

(event Input|EnhancedActionEvents|EnhancedInputActionIA_MoveForawrdBackward
  (params (ActionValue :type Float%20%28double-precision%29) (ElapsedSeconds :type Float%20%28double-precision%29) (TriggeredSeconds :type Float%20%28double-precision%29) (InputAction :type Input%20Action%20Object%20Reference :default "/Game/Inputs/IA_MoveForawrdBackward.IA_MoveForawrdBackward"))
  (Class|PawnMovementComponent|AddInputVector (Variables|Default|GetFloatingPawnMovement) (Math|Vector|MakeVector ActionValue 0.0 0.0) false))

(event Input|EnhancedActionEvents|EnhancedInputActionIA_MoveRightLeft
  (params (ActionValue :type Float%20%28double-precision%29) (ElapsedSeconds :type Float%20%28double-precision%29) (TriggeredSeconds :type Float%20%28double-precision%29) (InputAction :type Input%20Action%20Object%20Reference :default "/Game/Inputs/IA_MoveRightLeft.IA_MoveRightLeft"))
  (Class|PawnMovementComponent|AddInputVector (Variables|Default|GetFloatingPawnMovement) (Math|Vector|MakeVector 0.0 ActionValue 0.0) false))

(event Input|EnhancedActionEvents|EnhancedInputActionIA_LookWithMouse
  (params (ActionValue :type Vector%202D%20Structure) (ElapsedSeconds :type Float%20%28double-precision%29) (TriggeredSeconds :type Float%20%28double-precision%29) (InputAction :type Input%20Action%20Object%20Reference :default "/Game/Inputs/IA_LookWithMouse.IA_LookWithMouse"))
  (Pawn|Input|AddControllerYawInput (.x ActionValue))
  (Pawn|Input|AddControllerPitchInput (.y ActionValue)))

(event Input|EnhancedActionEvents|EnhancedInputActionIA_PrimaryFire
  (params (ActionValue :type Boolean) (ElapsedSeconds :type Float%20%28double-precision%29) (TriggeredSeconds :type Float%20%28double-precision%29) (InputAction :type Input%20Action%20Object%20Reference :default "/Game/Inputs/IA_PrimaryFire.IA_PrimaryFire"))
  (bind _projectile1 (Variables|Default|GetProjectile1))
  (bind _returnvalue (Transformation|GetWorldTransform _projectile1))
  (Utilities|FlowControl|Delay 0.2)
  (Game|SpawnActorfromClass "/Game/Blueprints/BP_Bullet.BP_Bullet_C" (Math|Transform|MakeTransform (.location _returnvalue) (.rotation _returnvalue) "1.000000,1.000000,1.000000") "Undefined" "MultiplyWithRoot" 0 0))

(event EventBeginPlay
  (CallFunction|SetRotatingParts))

(event EventPossessed
  (params (NewController :type Controller%20Object%20Reference))
  (bind _asplayer_controller (Utilities|Casting|CastToPlayerController NewController))
  (bind _output_get (Variables|Default|SetAs%20Player%20Controller _asplayer_controller))
  (Input|AddMappingContext (PlayerController|LocalPlayerSubsystems|GetEnhancedInputLocalPlayerSubsystem _output_get) "/Game/Inputs/IMC_PlayerInputs.IMC_PlayerInputs" 0 "(bIgnoreAllPressedKeysUntilRelease=True,bForceImmediately=False,bNotifyUserSettings=False)"))

(event EventTick
  (params (DeltaSeconds :type Float%20%28single-precision%29)))

(fn ConstructionScript)