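; Wave manager that spawns enemy waves in order from a data asset, starting at BeginPlay.
; Each wave waits its initial delay, then spawns each enemy group with random pauses before advancing, without waiting for deaths.
; Seeded-stream positions fall between LeftMax and RightMax, while boss waves use a fixed location.
; Spawns receive optional pickup drops and are flagged as last enemy in a final boss wave.
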(event Custom|SpawnNextWave
  (bind _leftmax (Variables|Default|GetLeftMax))
  (bind _currentwaveindex (Variables|Default|GetCurrentWaveIndex))
  (bind _waves (Variables|Default|GetWaves))
  (bind _returnvalue (Transformation|GetWorldLocation _leftmax))
  (bind _output (Utilities|Array|Get(acopy) _waves _currentwaveindex))
  (Math|Integer|IncrementInt _currentwaveindex
    (:%20%20
      (if (Utilities|Array|IsValidIndex _waves _currentwaveindex)
        (Utilities|FlowControl|Delay (.intialdelay _output))
        (if (.isbosswave _output)
          (Development|PrintString "boss is coming"))
        (Variables|Default|SetCurrentenemyData (.enemies _output))
        (bind _output_get (Variables|Default|SetCurrentenimiesIndex -1))
        (bind _result (Math|Integer|IncrementInt _output_get)
          (:%20%20
            (Development|PrintString (Utilities|String|Append "CurrentEnemy" (Utilities|String|ToString(Integer) _result)))
            (if (Utilities|Array|IsValidIndex (Variables|Default|GetCurrentenemyData) _result)
              (Variables|Default|SetMaxEnemyCount (.enemycount (Utilities|Array|Get(acopy) (Variables|Default|GetCurrentenemyData) (Variables|Default|GetCurrentenimiesIndex))))
              (bind _output_get_2 (Variables|Default|SetCurrentEnemyCount 0))
              (if (< _output_get_2 (Variables|Default|GetMaxEnemyCount)) :!label _label
                (Game|SpawnActorfromClass (.enemyclass (Utilities|Array|Get(acopy) (Variables|Default|GetCurrentenemyData) (Variables|Default|GetCurrentenimiesIndex))) (Math|Transform|MakeTransform (select (.isbosswave _output) "1400.000000,0.000000,0.000000" (Math|Vector|MakeVector (.x _returnvalue) (Math|Random|RandomFloatinRangefromStream (Variables|Default|GetStream_0) (.y _returnvalue) (.y (Transformation|GetWorldLocation (Variables|Default|GetRightMax)))) (.z _returnvalue))) (Transformation|GetWorldRotation _leftmax) "1.000000,1.000000,1.000000") "AlwaysSpawn" "MultiplyWithRoot" 0 (select (.candroppickup (Utilities|Array|Get(acopy) (Variables|Default|GetCurrentenemyData) (Variables|Default|GetCurrentenimiesIndex))) (.pickupclass (Utilities|Array|Get(acopy) (Variables|Default|GetCurrentenemyData) (Variables|Default|GetCurrentenimiesIndex))) 0) (and (.isbosswave _output) (== (Variables|Default|GetCurrentWaveIndex) (- (Variables|Default|GetNumberofWaves) 1))) 0)
                (Math|Integer|IncrementInt (Variables|Default|GetCurrentEnemyCount)
                  (:%20%20
                    (Utilities|FlowControl|Delay (Math|Random|RandomFloatinRangefromStream (Variables|Default|GetStream_0) 1.0 2.0))
                    (goto _label)))
                (else
                  (CallFunction|SpawnNextEnimiesinCurrentWave)))
              (else
                (CallFunction|SpawnNextWave)))))
        (else
          (Development|PrintString "no more waves in data assest to spawn"))))))

(event Custom|StartSpawningWaves
  (bind _leftmax (Variables|Default|GetLeftMax))
  (bind _currentwaveindex (Variables|Default|GetCurrentWaveIndex))
  (bind _waves (Variables|Default|GetWaves))
  (bind _returnvalue (Transformation|GetWorldLocation _leftmax))
  (bind _output (Utilities|Array|Get(acopy) _waves _currentwaveindex))
  (Utilities|FlowControl|Delay (.intialdelay _output))
  (if (.isbosswave _output)
    (Development|PrintString "boss is coming"))
  (Variables|Default|SetCurrentenemyData (.enemies _output))
  (bind _output_get (Variables|Default|SetCurrentenimiesIndex -1))
  (bind _result (Math|Integer|IncrementInt _output_get)
    (:%20%20
      (Development|PrintString (Utilities|String|Append "CurrentEnemy" (Utilities|String|ToString(Integer) _result)))
      (if (Utilities|Array|IsValidIndex (Variables|Default|GetCurrentenemyData) _result)
        (Variables|Default|SetMaxEnemyCount (.enemycount (Utilities|Array|Get(acopy) (Variables|Default|GetCurrentenemyData) (Variables|Default|GetCurrentenimiesIndex))))
        (bind _output_get_2 (Variables|Default|SetCurrentEnemyCount 0))
        (if (< _output_get_2 (Variables|Default|GetMaxEnemyCount)) :!label _label
          (Game|SpawnActorfromClass (.enemyclass (Utilities|Array|Get(acopy) (Variables|Default|GetCurrentenemyData) (Variables|Default|GetCurrentenimiesIndex))) (Math|Transform|MakeTransform (select (.isbosswave _output) "1400.000000,0.000000,0.000000" (Math|Vector|MakeVector (.x _returnvalue) (Math|Random|RandomFloatinRangefromStream (Variables|Default|GetStream_0) (.y _returnvalue) (.y (Transformation|GetWorldLocation (Variables|Default|GetRightMax)))) (.z _returnvalue))) (Transformation|GetWorldRotation _leftmax) "1.000000,1.000000,1.000000") "AlwaysSpawn" "MultiplyWithRoot" 0 (select (.candroppickup (Utilities|Array|Get(acopy) (Variables|Default|GetCurrentenemyData) (Variables|Default|GetCurrentenimiesIndex))) (.pickupclass (Utilities|Array|Get(acopy) (Variables|Default|GetCurrentenemyData) (Variables|Default|GetCurrentenimiesIndex))) 0) (and (.isbosswave _output) (== (Variables|Default|GetCurrentWaveIndex) (- (Variables|Default|GetNumberofWaves) 1))) 0)
          (Math|Integer|IncrementInt (Variables|Default|GetCurrentEnemyCount)
            (:%20%20
              (Utilities|FlowControl|Delay (Math|Random|RandomFloatinRangefromStream (Variables|Default|GetStream_0) 1.0 2.0))
              (goto _label)))
          (else
            (CallFunction|SpawnNextEnimiesinCurrentWave)))
        (else
          (CallFunction|SpawnNextWave))))))

(event Custom|SpawnNextEnimiesinCurrentWave
  (bind _leftmax (Variables|Default|GetLeftMax))
  (bind _currentenimiesindex (Variables|Default|GetCurrentenimiesIndex))
  (bind _currentwaveindex (Variables|Default|GetCurrentWaveIndex))
  (bind _waves (Variables|Default|GetWaves))
  (bind _currentenemydata (Variables|Default|GetCurrentenemyData))
  (bind _returnvalue (Transformation|GetWorldLocation _leftmax))
  (bind _output (Utilities|Array|Get(acopy) _waves _currentwaveindex))
  (bind _output_2 (Utilities|Array|Get(acopy) _currentenemydata _currentenimiesindex))
  (bind _result (Math|Integer|IncrementInt (stale Custom|SpawnNextWave _output_get))
    (:%20%20
      (Development|PrintString (Utilities|String|Append "CurrentEnemy" (Utilities|String|ToString(Integer) _result)))
      (if (Utilities|Array|IsValidIndex _currentenemydata _result)
        (Variables|Default|SetMaxEnemyCount (.enemycount _output_2))
        (bind _output_get (Variables|Default|SetCurrentEnemyCount 0))
        (if (< _output_get (Variables|Default|GetMaxEnemyCount)) :!label _label
          (Game|SpawnActorfromClass (.enemyclass _output_2) (Math|Transform|MakeTransform (select (.isbosswave _output) "1400.000000,0.000000,0.000000" (Math|Vector|MakeVector (.x _returnvalue) (Math|Random|RandomFloatinRangefromStream (Variables|Default|GetStream_0) (.y _returnvalue) (.y (Transformation|GetWorldLocation (Variables|Default|GetRightMax)))) (.z _returnvalue))) (Transformation|GetWorldRotation _leftmax) "1.000000,1.000000,1.000000") "AlwaysSpawn" "MultiplyWithRoot" 0 (select (.candroppickup _output_2) (.pickupclass _output_2) 0) (and (.isbosswave _output) (== (Variables|Default|GetCurrentWaveIndex) (- (Variables|Default|GetNumberofWaves) 1))) 0)
          (Math|Integer|IncrementInt (Variables|Default|GetCurrentEnemyCount)
            (:%20%20
              (Utilities|FlowControl|Delay (Math|Random|RandomFloatinRangefromStream (Variables|Default|GetStream_0) 1.0 2.0))
              (goto _label)))
          (else
            (CallFunction|SpawnNextEnimiesinCurrentWave)))
        (else
          (CallFunction|SpawnNextWave))))))

(event EventBeginPlay
  (Class|KismetMathLibrary|ResetRandomStream (Variables|Default|GetStream_0))
  (Variables|Default|SetWaves (Variables|/Game/Blueprints/PDA_SetofWaves.PDA_SetofWaves_C|GetWaves (Variables|Default|GetWavesDataAsset)))
  (Variables|Default|SetNumberofWaves (Utilities|Array|Length (Variables|/Game/Blueprints/PDA_SetofWaves.PDA_SetofWaves_C|GetWaves (Variables|Default|GetWavesDataAsset))))
  (CallFunction|StartSpawningWaves))

(fn ConstructionScript)