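; Player plane pawn for a shooter, with Enhanced Input movement, delayed bullet fire and an ammo-limited EMP.
; The EMP hits every BP_BaseEnemy, with clamped damage that grows with distance beyond a threshold.
; Overlaps deal contact damage, and sphere collision switches on shortly after spawn.
; Damage and pickups update health, reporting to HUD and controller; hits trigger shake, sound and red flash, and zero health triggers death.
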(event OnComponentBeginOverlap(Sphere)
  (params (OverlappedComponent :type Primitive%20Component%20Object%20Reference) (OtherActor :type Actor%20Object%20Reference) (OtherComp :type Primitive%20Component%20Object%20Reference) (OtherBodyIndex :type Integer) (bFromSweep :type Boolean) (SweepResult :type Hit%20Result%20Structure%20%28by%20ref%29))
  (Utilities|FlowControl|DoOnce false :!label _label
    (:Completed
      (Game|Damage|ApplyDamage OtherActor 25.0 0 0)
      (Utilities|FlowControl|Delay 0.4)
      (goto _label Reset))))

(event Custom|Apply%20camera%20shake
  (Camera|PlayWorldCameraShake "/Game/Blueprints/BP_Camerashakebase.BP_Camerashakebase_C" "0, 0, 0" 0.0 1e+03))

(event Custom|RotatingParts
  ;[0.15 0.02203 0 0.5] Add Rotation Later
)

(event Custom|Check%20Health
  (bind _asplayer_controller (Variables|Default|GetAsPlayer%20Controller)
    (:then
      (Class|BPIMyFlyingShump|SetHealthasPercent(Message) (HUD|GetHUD _asplayer_controller) (Math|Float|SafeDivide (Variables|Default|GetPlayerHealth) (Variables|Default|GetMax%20Health)))
      (if (== (Variables|Default|GetPlayerHealth) 0.0)
        (CallFunction|OnDeath)))
    (:else)))

(event Custom|OnDeath
  (Class|BPIMyFlyingShump|OnPlayerDeath(Message) (Game|GetPlayerController 0))
  (Niagara|SpawnSystematLocation "/Game/ParticlesSFX/FX_EnemyExplosion_System.FX_EnemyExplosion_System" (Transformation|GetActorLocation)))

(event Custom|FlashRedWhenHit
  (Rendering|Material|SetOverlayMaterial (Variables|Default|GetSM_plane) "/Game/Materials/M_OverlayWhenHit.M_OverlayWhenHit" :!class /Script/Engine.MeshComponent)
  (Utilities|FlowControl|Delay 0.3)
  (Rendering|Material|SetOverlayMaterial (Variables|Default|GetSM_plane) 0 :!class /Script/Engine.MeshComponent))

(event Custom|Update%20Hud
  ;[0.15 0.15 0.15 0.5] HUD
  (Class|BPIMyFlyingShump|SetHealthasPercent(Message) (HUD|GetHUD (Variables|Default|GetAsPlayer%20Controller)) (Math|Float|SafeDivide (Variables|Default|GetPlayerHealth) (Variables|Default|GetMax%20Health))))

(event Custom|DeployEMP
  (bind _outactors (Actor|GetAllActorsOfClass "/Game/Blueprints/BP_BaseEnemy.BP_BaseEnemy_C"))
  (for _array_element _outactors
    (bind _returnvalue (Game|SpawnActorfromClass "/Game/Blueprints/BP_EMP_SFX.BP_EMP_SFX_C" (Math|Transform|MakeTransform "0, 0, 0" "0, 0, 0" "1.000000,1.000000,1.000000") "AlwaysSpawn" "MultiplyWithRoot" 0 0))
    (Transformation|AttachActorToActor _returnvalue _array_element "None" "KeepRelative" "KeepWorld" "KeepWorld" true)
    (Game|Damage|ApplyDamage _array_element (* (Math|Float|Clamp(Float) (- (Math|Vector|Distance(Vector) (Transformation|GetActorLocation _array_element) (Transformation|GetActorLocation)) 4.7e+02) 0.0 1.2e+03) 0.5) 0 0)))

(event Input|EnhancedActionEvents|EnhancedInputActionIA_MoveForawrdBackward
  (params (ActionValue :type Float%20%28double-precision%29) (ElapsedSeconds :type Float%20%28double-precision%29) (TriggeredSeconds :type Float%20%28double-precision%29) (InputAction :type Input%20Action%20Object%20Reference :default "/Game/Inputs/IA_MoveForawrdBackward.IA_MoveForawrdBackward"))
  (Class|PawnMovementComponent|AddInputVector (Variables|Default|GetFloatingPawnMovement) (Math|Vector|MakeVector ActionValue 0.0 0.0) false))

(event Input|EnhancedActionEvents|EnhancedInputActionIA_MoveRightLeft
  (params (ActionValue :type Float%20%28double-precision%29) (ElapsedSeconds :type Float%20%28double-precision%29) (TriggeredSeconds :type Float%20%28double-precision%29) (InputAction :type Input%20Action%20Object%20Reference :default "/Game/Inputs/IA_MoveRightLeft.IA_MoveRightLeft"))
  (Class|PawnMovementComponent|AddInputVector (Variables|Default|GetFloatingPawnMovement) (Math|Vector|MakeVector 0.0 ActionValue 0.0) false))

(event Input|EnhancedActionEvents|EnhancedInputActionIA_PrimaryFire
  (params (ActionValue :type Boolean) (ElapsedSeconds :type Float%20%28double-precision%29) (TriggeredSeconds :type Float%20%28double-precision%29) (InputAction :type Input%20Action%20Object%20Reference :default "/Game/Inputs/IA_PrimaryFire.IA_PrimaryFire"))
  (bind _arrow (Variables|Default|GetArrow))
  (bind _returnvalue (Transformation|GetWorldTransform _arrow))
  ;[0.15 0.01181 0 0.5] Primary Shooting
  (Utilities|FlowControl|Delay 0.2)
  (Game|SpawnActorfromClass "/Game/Blueprints/BP_2dPlayerBullet.BP_2dPlayerBullet_C" (Math|Transform|MakeTransform (.location _returnvalue) (.rotation _returnvalue) "1.000000,1.000000,1.000000") "Undefined" "MultiplyWithRoot" 0 0)
  (Audio|PlaySound2D "/Game/Sci-Fi_Shots_Pack2_Game_Of_Weapons/Wave/SciFi_Shot_P2__66_.SciFi_Shot_P2__66_" 1.0 1.0 0.0 0 0))

(event Input|EnhancedActionEvents|EnhancedInputActionIA_SecondaryFire
  (params (ActionValue :type Boolean) (ElapsedSeconds :type Float%20%28double-precision%29) (TriggeredSeconds :type Float%20%28double-precision%29) (InputAction :type Input%20Action%20Object%20Reference :default "/Game/Inputs/IA_SecondaryFire.IA_SecondaryFire"))
  (:Completed
    (Utilities|FlowControl|Delay 0.2)
    (if (> (Variables|Default|GetAmmo_EMP) 0)
      (bind _result (Math|Integer|DecrementInt (Variables|Default|GetAmmo_EMP))
        (:%20%20
          (Class|BPIMyFlyingShump|SetEMP(Message) (HUD|GetHUD (Pawn|GetLocalViewingPlayerController)) _result)
          (CallFunction|DeployEMP))))))

(event EventBeginPlay
  (Utilities|FlowControl|Delay 2.0)
  (Collision|SetCollisionProfileName (Variables|Default|GetSphere) "Player" true :!class /Script/Engine.PrimitiveComponent)
  (Collision|SetCollisionEnabled (Variables|Default|GetSphere) "QueryAndPhysics"))

(event Game|Damage|EventAnyDamage
  (params (Damage :type Float%20%28single-precision%29) (DamageType :type Damage%20Type%20Object%20Reference) (InstigatedBy :type Controller%20Object%20Reference) (DamageCauser :type Actor%20Object%20Reference))
  (Variables|Default|SetPlayerHealth (Math|Float|Clamp(Float) (- (Variables|Default|GetPlayerHealth) Damage) 0.0 (Variables|Default|GetMax%20Health)))
  (CallFunction|ApplyCameraShake)
  (Audio|PlaySound2D "/Game/Sci-Fi_Shots_Pack2_Game_Of_Weapons/Wave/SciFi_Shot_P2__59_.SciFi_Shot_P2__59_" 1.0 1.0 0.0 0 0)
  (CallFunction|FlashRedwhenHit)
  (CallFunction|CheckHealth))

(event Collision|EventActorBeginOverlap
  (params (OtherActor :type Actor%20Object%20Reference))
  (Game|Damage|ApplyDamage OtherActor (Variables|Default|GetPlayerHealth) 0 0))

(event EventPossessed
  (params (NewController :type Controller%20Object%20Reference))
  (bind _asplayer_controller (Utilities|Casting|CastToPlayerController NewController))
  (bind _output_get (Variables|Default|SetAsPlayer%20Controller _asplayer_controller))
  (Input|AddMappingContext (PlayerController|LocalPlayerSubsystems|GetEnhancedInputLocalPlayerSubsystem _output_get) "/Game/Inputs/IMC_PlayerInputs.IMC_PlayerInputs" 0 "(bIgnoreAllPressedKeysUntilRelease=True,bForceImmediately=False,bNotifyUserSettings=False)")
  (CallFunction|CheckHealth))

(event EventOnPickup
  (params (AddHealth :type Float%20%28double-precision%29) (AddMaxHealth :type Float%20%28double-precision%29) (AddLives :type Integer) (SetMaxLives :type Integer) (AddScore :type Integer) (SetShootingMode :type Integer) (AddShooting%20Mode :type Integer) (EMPAmmo :type Integer))
  (Utilities|FlowControl|Sequence
    (:then_0
      (Variables|Default|SetMax%20Health (+ AddMaxHealth (Variables|Default|GetMax%20Health))))
    (:then_1
      (Variables|Default|SetPlayerHealth (Math|Float|Clamp(Float) (+ AddHealth (Variables|Default|GetPlayerHealth)) 0.0 (Variables|Default|GetMax%20Health)))
      (CallFunction|CheckHealth)
      (Class|BPIMyFlyingShump|AddPlayerLives(Message) (Pawn|GetController) AddLives))
    (:then_2
      (bind _output_get (Variables|Default|SetAmmo_EMP (+ EMPAmmo (Variables|Default|GetAmmo_EMP))))
      (Class|BPIMyFlyingShump|SetEMP(Message) (HUD|GetHUD (Pawn|GetLocalViewingPlayerController)) _output_get))))

(event Input|KeyboardEvents|DebugKeyP
  (params (Key :type Key%20Structure :default "None") (ActionValue :type Input%20Action%20Value%20Structure))
  (:Pressed
    (Class|BPIMyFlyingShump|AddPlayerLives(Message) (Pawn|GetController) -1)))

(event Input|KeyboardEvents|DebugKeyO
  (params (Key :type Key%20Structure :default "None") (ActionValue :type Input%20Action%20Value%20Structure)))

(fn ConstructionScript)