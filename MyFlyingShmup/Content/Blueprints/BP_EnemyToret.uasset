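; Enemy turret Blueprint that swings its shooting arrow in yaw based on the player pawn's position, starting at BeginPlay.
; The FireSequence timeline sets the arrow's relative yaw each update to the look-at yaw scaled by a curve, plus a stored ShootingDirection.
; Its Start Rotating event track captures the arrow's current yaw as that offset.
; No projectile or damage logic appears in these graphs.
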(event Custom|StartShooting
  (bind _yawmultiplire (Timeline|FireSequence PlayFromStart)
    (:Update
      (Transformation|SetRelativeRotation (Variables|Default|GetArrowofShooting) (Math|Rotator|MakeRotator 0.0 0.0 (+ (* _yawmultiplire (.yaw (Math|Rotator|FindLookatRotation (Transformation|GetActorLocation) (Transformation|GetActorLocation (Game|Player|GetPlayerPawn 0))))) 0.0 (Variables|Default|GetShootingDirection))) false false))
    (:Start%20Rotating%20
      (Variables|Default|SetShootingDirection (.yaw (Variables|/Script/Engine.SceneComponent|GetRelativeRotation (Variables|Default|GetArrowofShooting)))))))

(event EventBeginPlay
  (|CallParentFunction)
  (CallFunction|StartShooting))

(fn ConstructionScript
  (|CallParentFunction))