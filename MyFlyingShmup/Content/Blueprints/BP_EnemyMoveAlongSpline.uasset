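; Enemy actor that moves along its own spline, starting on BeginPlay.
; A slowed timeline supplies the time used to sample the spline's local-space location, without constant velocity.
; Each update makes the cached initial transform relative to that location, so the spline point is subtracted from the start position rather than added.
; Only position follows the spline, as the sampled transform carries no rotation and unit scale.
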(event EventBeginPlay
  (|CallParentFunction)
  (Components|Timeline|SetPlayRate (Variables|Default|GetTimeline) 0.1)
  (Variables|Default|SetIntialTransform (Transformation|GetActorTransform))
  (bind _newtrack_0 (Timeline|Timeline PlayFromStart)
    (:Update
      (Transformation|SetActorTransform (Math|Transform|MakeRelativeTransform (Variables|Default|GetIntialTransform) (Math|Transform|MakeTransform (Spline|GetLocationatTime (Variables|Default|GetSpline) _newtrack_0 "Local" false)))))))

(fn ConstructionScript
  (|CallParentFunction))