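; BP_EnemyHoming is a homing enemy actor that chases the player pawn through its ProjectileMovement component.
; On BeginPlay it sets the player pawn's root component as the homing target.
; Each Tick it overwrites the projectile velocity with a fixed-speed vector built from the look-at yaw toward the player, so the steering is purely horizontal.
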(event EventTick
  (params (DeltaSeconds :type Float%20%28single-precision%29))
  (Variables|/Script/Engine.MovementComponent|SetVelocity (Variables|Default|GetProjectileMovement) (* (Math|Rotator|GetRotationXVector (Math|Rotator|MakeRotator 0.0 0.0 (.yaw (Math|Rotator|FindLookatRotation (Transformation|GetActorLocation) (Transformation|GetActorLocation (Game|Player|GetPlayerPawn 0)))))) "100.000000,100.000000,100.000000")))

(event EventBeginPlay
  (Variables|/Script/Engine.ProjectileMovementComponent|SetHomingTargetComponent (Variables|Default|GetProjectileMovement) (Variables|/Script/Engine.Actor|GetRootComponent (Game|Player|GetPlayerPawn 0))))

(fn ConstructionScript
  (|CallParentFunction))