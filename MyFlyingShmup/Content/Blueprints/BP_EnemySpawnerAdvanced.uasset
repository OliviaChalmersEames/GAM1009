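; BP_EnemySpawnerAdvanced is an enemy spawner meant to place BP_EnemyA at a random Y between two arrow components.
; SpawnEnemy and QueTimer form a self-rescheduling loop with random delays, using the left arrow for X, Z and rotation.
; Nothing live starts that loop: BeginPlay loops a timer on the empty GetRandomValue event and resets a random stream that the random range calls do not use.
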(event Custom|Que%20Timer
  (Utilities|Time|SetTimerbyEvent (delegate Custom|Spawn%20Enemy) (Math|Random|RandomFloatinRange 1.0 3.0)))

(event Custom|Spawn%20Enemy
  (bind _arrowleft (Variables|Default|GetArrowLeft))
  (bind _returnvalue (Transformation|GetWorldLocation _arrowleft))
  (Game|SpawnActorfromClass "/Game/Blueprints/BP_EnemyA.BP_EnemyA_C" (Math|Transform|MakeTransform (Math|Vector|MakeVector (.x _returnvalue) (Math|Random|RandomFloatinRange (.y (Transformation|GetWorldLocation (Variables|Default|GetArrowRight))) (.y _returnvalue)) (.z _returnvalue)) (Transformation|GetWorldRotation _arrowleft) "1.000000,1.000000,1.000000") "Undefined" "MultiplyWithRoot" 0 0)
  (CallFunction|QueTimer))

(event Custom|GetRandomValue)

(event EventBeginPlay
  (Utilities|Time|SetTimerbyEvent (delegate Custom|GetRandomValue) 1.0 true)
  (Class|KismetMathLibrary|ResetRandomStream (Variables|Default|GetStream)))

(fn ConstructionScript)