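; BP_Base_Pickup is a base pickup actor that homes in on an overlapping actor and hands it configurable bonuses.
; Overlapping the outer sphere turns on projectile homing toward that actor's root component and sets the max speed.
; Overlapping the inner sphere sends OnPickupMessage with health, lives, score, shooting mode and EMP ammo values, then destroys the pickup.
; Neither overlap filters by actor type.
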(event OnComponentBeginOverlap(outersphere)
  (params (OverlappedComponent :type Primitive%20Component%20Object%20Reference) (OtherActor :type Actor%20Object%20Reference) (OtherComp :type Primitive%20Component%20Object%20Reference) (OtherBodyIndex :type Integer) (bFromSweep :type Boolean) (SweepResult :type Hit%20Result%20Structure%20%28by%20ref%29))
  (bind _projectilemovement (Variables|Default|GetProjectileMovement))
  (Variables|/Script/Engine.ProjectileMovementComponent|SetHomingTargetComponent _projectilemovement (Variables|/Script/Engine.Actor|GetRootComponent OtherActor))
  (Variables|/Script/Engine.ProjectileMovementComponent|SetbIsHomingProjectile _projectilemovement true)
  (Variables|/Script/Engine.ProjectileMovementComponent|SetMaxSpeed _projectilemovement 1e+03))

(event OnComponentBeginOverlap(Innersphere)
  (params (OverlappedComponent :type Primitive%20Component%20Object%20Reference) (OtherActor :type Actor%20Object%20Reference) (OtherComp :type Primitive%20Component%20Object%20Reference) (OtherBodyIndex :type Integer) (bFromSweep :type Boolean) (SweepResult :type Hit%20Result%20Structure%20%28by%20ref%29))
  (Class|BPIMyFlyingShump|OnPickup(Message) OtherActor (Variables|Default|GetAddHealthBonus) (Variables|Default|GetSetHealthBonus) (Variables|Default|GetSetLivesbonus) (Variables|Default|GetSetLivesLimitBonus) (Variables|Default|GetSetScore) (Variables|Default|GetSetShootingMode) (Variables|Default|GetAddShootingModeIndex) (Variables|Default|GetAddEMPAmmo))
  (Actor|DestroyActor))

(fn ConstructionScript)