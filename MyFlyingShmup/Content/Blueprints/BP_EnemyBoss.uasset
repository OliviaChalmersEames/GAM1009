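; Enemy boss actor that moves along a path while firing BP_Enemybullet projectiles.
; On BeginPlay a half-speed timeline drives its transform from spline positions, then a second timeline shifts it along Y.
; Looping timers spawn bullets at the Arrow component, with a shot sound played when shooting starts.
; BeginPlay calls that shooting event twice; the parallel Arrow1 shooting event is never called here.
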(event Custom|SpawnBullet
  (bind _arrow (Variables|Default|GetArrow))
  (bind _returnvalue (Transformation|GetWorldTransform _arrow))
  (Game|SpawnActorfromClass "/Game/Blueprints/BP_Enemybullet.BP_Enemybullet_C" (Math|Transform|MakeTransform (.location _returnvalue) (.rotation _returnvalue) "1.000000,1.000000,1.000000") "Undefined" "MultiplyWithRoot" 0 0))

(event Custom|Begin_Regular_Shooting
  (Utilities|Time|SetTimerbyEvent (delegate Custom|Spawn_Bullet) 2.0 true)
  (Audio|SpawnSound2D "/Game/Sci-Fi_Shots_Pack2_Game_Of_Weapons/Cue/SciFi_Shot_P2__78__Cue.SciFi_Shot_P2__78__Cue" 1.0 1.0 0.0 0))

(event Custom|Spawn_Bullet
  (bind _arrow1 (Variables|Default|GetArrow1))
  (bind _returnvalue (Transformation|GetWorldTransform _arrow1))
  (Game|SpawnActorfromClass "/Game/Blueprints/BP_Enemybullet.BP_Enemybullet_C" (Math|Transform|MakeTransform (.location _returnvalue) (.rotation _returnvalue) "1.000000,1.000000,1.000000") "Undefined" "MultiplyWithRoot" 0 0))

(event Custom|BeginRegularShooting
  (Utilities|Time|SetTimerbyEvent (delegate Custom|SpawnBullet) 2.0 true)
  (Audio|SpawnSound2D "/Game/Sci-Fi_Shots_Pack2_Game_Of_Weapons/Cue/SciFi_Shot_P2__78__Cue.SciFi_Shot_P2__78__Cue" 1.0 1.0 0.0 0))

(event EventBeginPlay
  (CallFunction|BeginRegularShooting)
  (CallFunction|BeginRegularShooting)
  (|CallParentFunction)
  (Components|Timeline|SetPlayRate (Variables|Default|GetTimeline) 0.5)
  (Variables|Default|SetIntialTransform (Transformation|GetActorTransform))
  (bind _progress (Timeline|Timeline PlayFromStart)
    (:Update
      (bind _spline (Variables|Default|GetSpline)
        (:then
          (Transformation|SetActorTransform (Math|Transform|MakeRelativeTransform (Variables|Default|GetIntialTransform) (Math|Transform|MakeTransform (Spline|GetLocationatTime _spline _progress "Local" true))) true))
        (:else)))
    (:Finished
      (Variables|Default|SetIntialTransform (Transformation|GetActorTransform))
      (bind _time (Timeline|LefttoRight PlayFromStart)
        (:Update
          (Transformation|SetActorTransform (Math|Transform|MakeRelativeTransform (Math|Transform|MakeTransform (Math|Vector|MakeVector 0.0 (* _time 8e+02) 0.0) "0, 0, 0" "1.000000,1.000000,1.000000") (Variables|Default|GetIntialTransform)) true))))))

(fn ConstructionScript
  (|CallParentFunction))