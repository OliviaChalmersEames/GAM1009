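; BP_EnemyA is an enemy actor that automatically fires BP_Enemybullet projectiles.
; On BeginPlay it starts a looping timer that spawns a bullet at its Arrow component's transform, playing the shot sound only when the timer starts.
; Two hit-flash events, neither triggered within this graph, apply an overlay material to its meshes, then re-apply the same material after a delay instead of clearing it.
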(event Custom|Begin_Regular_Shooting
  (Utilities|Time|SetTimerbyEvent (delegate Custom|Spawn_Bullet) 2.0 true)
  (Audio|SpawnSound2D "/Game/Sci-Fi_Shots_Pack2_Game_Of_Weapons/Cue/SciFi_Shot_P2__78__Cue.SciFi_Shot_P2__78__Cue" 1.0 1.0 0.0 0))

(event Custom|Spawn_Bullet
  (bind _arrow (Variables|Default|GetArrow))
  (bind _returnvalue (Transformation|GetWorldTransform _arrow))
  (Game|SpawnActorfromClass "/Game/Blueprints/BP_Enemybullet.BP_Enemybullet_C" (Math|Transform|MakeTransform (.location _returnvalue) (.rotation _returnvalue) "1.000000,1.000000,1.000000") "Undefined" "MultiplyWithRoot" 0 0))

(event Custom|FlashRedWhenHit
  (Rendering|Material|SetOverlayMaterial (Variables|Default|Getscene1) "/Game/Materials/M_OverlayWhenHit.M_OverlayWhenHit" :!class /Script/Engine.MeshComponent)
  (Utilities|FlowControl|Delay 0.3)
  (Rendering|Material|SetOverlayMaterial (Variables|Default|Getscene1) "/Game/Materials/M_OverlayWhenHit.M_OverlayWhenHit" :!class /Script/Engine.MeshComponent))

(event Custom|CustomEvent
  (bind _scene1 (Variables|Default|Getscene1)
    (:then
      (Rendering|Material|SetOverlayMaterial _scene1 "/Game/Materials/M_OverlayWhenHit.M_OverlayWhenHit" :!class /Script/Engine.MeshComponent)
      (Utilities|FlowControl|Delay 0.2)
      (bind _scene1_2 (Variables|Default|Getscene1)
        (:then
          (Rendering|Material|SetOverlayMaterial _scene1_2 "/Game/Materials/M_OverlayWhenHit.M_OverlayWhenHit" :!class /Script/Engine.MeshComponent))
        (:else)))
    (:else)))

(event EventBeginPlay
  (CallFunction|BeginRegularShooting))

(fn ConstructionScript
  (|CallParentFunction))