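; Base enemy Blueprint that damages actors it touches, awards the player score when hit or killed, and can end the level.
; Actor overlap deals damage equal to current health, while the Sphere deals fixed damage behind a timed DoOnce cooldown.
; Incoming damage updates the health widget, plays a sound and briefly flashes an overlay material.
; Zero health triggers an explosion, pickup drop and, for the level's last enemy, the end screen.
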(event OnComponentBeginOverlap(Sphere)
  (params (OverlappedComponent :type Primitive%20Component%20Object%20Reference) (OtherActor :type Actor%20Object%20Reference) (OtherComp :type Primitive%20Component%20Object%20Reference) (OtherBodyIndex :type Integer) (bFromSweep :type Boolean) (SweepResult :type Hit%20Result%20Structure%20%28by%20ref%29))
  (Utilities|FlowControl|DoOnce false :!label _label
    (:Completed
      (Game|Damage|ApplyDamage OtherActor 25.0 0 0)
      (Utilities|FlowControl|Delay 0.4)
      (goto _label Reset))))

(event Custom|SpawnExplosion
  (Niagara|SpawnSystematLocation "/Game/ParticlesSFX/FX_EnemyExplosion_System.FX_EnemyExplosion_System" (Transformation|GetActorLocation)))

(event Custom|check%20health
  (if (== (Variables|Default|GetHealth) 0.0)
    (Class|BPIMyFlyingShump|AddScore(Message) (Game|GetPlayerController 0) (Variables|Default|GetMax%20Health))
    (CallFunction|OnDeath)))

(event Custom|on%20death
  (bind _returnvalue (Transformation|GetActorTransform))
  (bind _islastenemeyoflevel (Variables|Default|GetIsLastEnemeyOfLevel))
  (Audio|PlaySound2D "/Game/Sci-Fi_Shots_Pack2_Game_Of_Weapons/Wave/SciFi_Shot_P2__91_.SciFi_Shot_P2__91_" 1.0 1.0 0.0 0 0)
  (CallFunction|SpawnExplosion)
  (Game|SpawnActorfromClass (Variables|Default|GetPickUptoDroponDeath) (Math|Transform|MakeTransform (.location _returnvalue) (.rotation _returnvalue) "1.000000,1.000000,1.000000") "Undefined" "MultiplyWithRoot" 0 0)
  (if _islastenemeyoflevel
    (Class|BPIMyFlyingShump|ShowEndScreen(Message) (Game|GetPlayerController 0) _islastenemeyoflevel))
  (Actor|DestroyActor))

(event Custom|FlashRedOverlayMaterial
  (bind _mesh (Variables|Default|GetMesh)
    (:then
      (Rendering|Material|SetOverlayMaterial _mesh "/Game/Materials/M_OverlayWhenHit.M_OverlayWhenHit" :!class /Script/Engine.MeshComponent)
      (Utilities|FlowControl|Delay 0.2)
      (bind _mesh_2 (Variables|Default|GetMesh)
        (:then
          (Rendering|Material|SetOverlayMaterial _mesh_2 0 :!class /Script/Engine.MeshComponent))
        (:else)))
    (:else)))

(event EventBeginPlay
  (Variables|Default|SetHealth (Variables|Default|GetMax%20Health)))

(event Collision|EventActorBeginOverlap
  (params (OtherActor :type Actor%20Object%20Reference))
  (Game|Damage|ApplyDamage OtherActor (Variables|Default|GetHealth) 0 0))

(event Game|Damage|EventAnyDamage
  (params (Damage :type Float%20%28single-precision%29) (DamageType :type Damage%20Type%20Object%20Reference) (InstigatedBy :type Controller%20Object%20Reference) (DamageCauser :type Actor%20Object%20Reference))
  (Class|BPIMyFlyingShump|AddScore(Message) (Game|GetPlayerController 0) Damage)
  (Variables|Default|SetHealth (Math|Float|Clamp(Float) (- (Variables|Default|GetHealth) Damage) 0.0 (Variables|Default|GetMax%20Health)))
  (Class|BPIMyFlyingShump|SetHealthasPercent(Message) (UserInterface|GetUserWidgetObject (Variables|Default|GetWidget)) (Math|Float|SafeDivide (Variables|Default|GetHealth) (Variables|Default|GetMax%20Health)))
  (CallFunction|CheckHealth)
  (Audio|PlaySound2D "/Game/Sci-Fi_Shots_Pack2_Game_Of_Weapons/Cue/SciFi_Shot_P2__119__Cue.SciFi_Shot_P2__119__Cue" 1.0 1.0 0.0 0 0)
  (CallFunction|FlashRedOverlayMaterial))

(fn ConstructionScript)